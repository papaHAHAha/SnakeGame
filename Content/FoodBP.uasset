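; FoodBP is a food actor with a Sphere component and a FoodType, apparently a collectible with visual variants.
; BeginPlay only sets the Special, Regular and SpeedUp material variables from values of the same name.
; A switch on FoodType that sets the Sphere material for Regular and Special food is disconnected and never runs.
; Tick, overlap and construction logic are empty.
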(event `self.ReceiveBeginPlay`
  (set `self.SpecialMaterial` (`self.SpecialMaterial_`))
  (set `self.RegularMaterial` (`self.RegularMaterial_`))
  (set `self.SpeedUpMaterial` (`self.SpeedUpMaterial_`)))

(event `self.ReceiveTick`
  (params (DeltaSeconds :type "Float (single-precision)")))

(fn `UserConstructionScript`)